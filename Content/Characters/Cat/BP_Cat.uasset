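; Playable cat character that links its health bar widget to itself and uses the Gameplay Ability System for a punch attack.
; On the server, it grants GA_Punch, retrying until the PlayerState is available, and routes death to the game mode and a client montage.
; Melee goes from the locally controlled client to a server sphere overlap with debug drawing, sending an Ability.Damage event to the instigator per pawn hit.
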(event `self.ReceiveBeginPlay`
  (`|ExecutionSequence`
    (:`then_0`
      (bind _aswbp_health_bar (cast `/Game/Widgets/WBP_HealthBar` (`WidgetComponent.GetUserWidgetObject` (`self.HPBar`))))
      (set `/Game/Widgets/WBP_HealthBar.PBOwner` self _aswbp_health_bar))
    (:`then_1`
      (if (`KismetSystemLibrary.IsServer`)
        (`|ExecutionSequence`
          (:`then_0`
            (bind _aspbplayer_state (cast `PBPlayerState` (`self.PlayerState`) :!label _label)
              (:`then`
                (`PBAbilitySystemComponent.AddCharacterAbilities` (`PBPlayerState.PBASC` _aspbplayer_state) (`|MakeArray` "/Game/GAS/Abilities/GA_Punch.GA_Punch_C" :!type "GameplayAbility Class Reference")))
              (:`CastFailed`
                (`KismetSystemLibrary.Delay` 0.2)
                (goto _label))))
          (:`then_1`
            (add `self.OnDeath` (delegate `HandleDeath`))))))))

(event `ClientDeath`
  (`|PlayMontage` null))

(event `HandleDeath`
  (bind _aspbgame_mode (cast `PBGameMode` (`GameplayStatics.GetGameMode`)))
  (`/Game/GM_Base.PlayerDeath` _aspbgame_mode self)
  (`self.ClientDeath`))

(event `HandleMelee`
  (if (`self.IsLocallyControlled`)
    (`self.ServerHandleMelee`)))

(event `ServerHandleMelee`
  (bind _returnvalue (`self.GetInstigator`))
  (bind _returnvalue_2 (+ (`self.K2_GetActorLocation`) (* (`self.GetActorForwardVector`) 60.0)))
  (`KismetSystemLibrary.DrawDebugSphere` _returnvalue_2 20.0 12 (struct :`R` 1.0 :`G` 1.0 :`B` 1.0 :`A` 1.0) 5.0 1.0)
  (bind _outactors (`KismetSystemLibrary.SphereOverlapActors` _returnvalue_2 20.0 (`|MakeArray` "ObjectTypeQuery3" :!type "EObjectTypeQuery Enum") null (`|MakeArray` self :!type "Actor Object Reference")))
  (for _array_element _outactors
    (`AbilitySystemBlueprintLibrary.SendGameplayEventToActor` _returnvalue (struct :`TagName` "Ability.Damage") (make `GameplayEventData` (struct) _returnvalue _array_element null null (struct) (struct) (struct) 0.0 (`AbilitySystemBlueprintLibrary.AbilityTargetDataFromActor` _array_element)))))

(fn `UserConstructionScript`)