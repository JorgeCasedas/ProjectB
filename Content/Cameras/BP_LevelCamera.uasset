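; BP_LevelCamera is a shared level camera that follows every BP_Raphtalia actor.
; Each Tick it moves to their averaged location, then sets spring arm length from the ratio of current to initial player spread, clamped.
; The zoom runs only when the initial distance is nonzero.
; View-target setup, initial capture and maximum pairwise distance measurement are disconnected, so the graph never updates those distances.
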(event `self.ReceiveBeginPlay`)

(event `self.ReceiveTick`
  (params (DeltaSeconds :type "Float (single-precision)"))
  (`self.RepositionCamera`)
  (`self.K2_SetActorLocation` (`self.MidPoint`))
  (`self.ReZoomCamera`))

(event `RepositionCamera`
  (set `self.X` 0.0)
  (set `self.Y` 0.0)
  (set `self.Z` 0.0)
  (bind _outactors (`GameplayStatics.GetAllActorsOfClass` "/Game/Characters/Raphtalia_Root/BP_Raphtalia.BP_Raphtalia_C"))
  (for _array_element _outactors
    (bind (_returnvalue_x _returnvalue_y _returnvalue_z) (`KismetMathLibrary.BreakVector` (`self.K2_GetActorLocation` _array_element)))
    (set `self.X` (+ (`self.X`) _returnvalue_x))
    (set `self.Y` (+ (`self.Y`) _returnvalue_y))
    (set `self.Z` (+ (`self.Z`) _returnvalue_z)))
  (bind _returnvalue (`KismetArrayLibrary.Array_Length` _outactors))
  (set `self.MidPoint` (`KismetMathLibrary.MakeVector` (/ (`self.X`) _returnvalue) (/ (`self.Y`) _returnvalue) (/ (`self.Z`) _returnvalue))))

(event `ReZoomCamera`
  (if (!= (`self.InitPlayersDistance_0`) 0.0)
    (set `SpringArmComponent.TargetArmLength` (`KismetMathLibrary.FClamp` (* (`self.InitArmLength`) (/ (`self.ActualPlayersDistance`) (`self.InitPlayersDistance_0`))) (`self.MinArmLength_0`) (`self.MaxArmLength_0`)) (`self.SpringArm`))))

(fn `UserConstructionScript`)