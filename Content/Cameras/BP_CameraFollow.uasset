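; Camera actor that follows the horizontal position of an assigned actor and serves as the player's view.
; On BeginPlay it casts ActorToFollow to Character and makes itself the view target of that character's PlayerController with a short blend.
; Each Tick, while the target is valid, it snaps its location to the target's X and Y without smoothing, ignoring the target's height and rotation.
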(event `self.ReceiveBeginPlay`
  (`PlayerController.SetViewTargetWithBlend` (cast `PlayerController` (`Pawn.GetController` (cast `Character` (`self.ActorToFollow`) :!pure true)) :!pure true) self 0.1 "VTBlend_Linear" 0.1 true))

(event `self.ReceiveTick`
  (params (DeltaSeconds :type "Float (single-precision)"))
  (bind _actortofollow (`self.ActorToFollow`))
  (bind (_returnvalue_x _returnvalue_y) (`KismetMathLibrary.BreakVector` (`self.K2_GetActorLocation` _actortofollow)))
  (`/Engine/EditorBlueprintResources/StandardMacros.IsValid` _actortofollow
    (:`Is Valid`
      (`self.K2_SetActorLocation` (`KismetMathLibrary.MakeVector` _returnvalue_x _returnvalue_y)))))

(fn `UserConstructionScript`)