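; Shared camera that becomes player 0's view target at BeginPlay and keeps all BP_Raphtalia actors framed.
; Each tick it moves to their average position and rescales the spring arm by their largest pairwise distance.
; Zoom is proportional to a baseline arm length and spread captured after a short startup delay, clamped between minimum and maximum lengths.
; Zooming is skipped while the baseline spread is zero.
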(event `self.ReceiveBeginPlay`
  (`PlayerController.SetViewTargetWithBlend` (`GameplayStatics.GetPlayerController` 0) self 0.1 "VTBlend_Linear" 0.1 true)
  (`KismetSystemLibrary.Delay` 3.0)
  (set `self.InitArmLength` (`SpringArmComponent.TargetArmLength` (`self.SpringArm`)))
  (`self.GetMaxPlayersDistance`)
  (set `self.InitPlayersDistance` (`self.ActualPlayersDistance`)))

(event `self.ReceiveTick`
  (params (DeltaSeconds :type "Float (single-precision)"))
  (`self.RepositionCamera`)
  (`self.K2_SetActorLocation` (`self.MidPoint`))
  (`self.ReZoomCamera`))

(event `RepositionCamera`
  (set `self.X` 0.0)
  (set `self.Y` 0.0)
  (set `self.Z` 0.0)
  (bind _outactors (`GameplayStatics.GetAllActorsOfClass` "/Game/Characters/Raphtalia_Root/BP_Raphtalia.BP_Raphtalia_C"))
  (for _array_element _outactors
    (bind (_returnvalue_x _returnvalue_y _returnvalue_z) (`KismetMathLibrary.BreakVector` (`self.K2_GetActorLocation` _array_element)))
    (set `self.X` (+ (`self.X`) _returnvalue_x))
    (set `self.Y` (+ (`self.Y`) _returnvalue_y))
    (set `self.Z` (+ (`self.Z`) _returnvalue_z)))
  (bind _returnvalue (`KismetArrayLibrary.Array_Length` _outactors))
  (set `self.MidPoint` (`KismetMathLibrary.MakeVector` (/ (`self.X`) _returnvalue) (/ (`self.Y`) _returnvalue) (/ (`self.Z`) _returnvalue))))

(event `GetMaxPlayersDistance`
  (set `self.ActualPlayersDistance` 0.0)
  (bind _outactors (`GameplayStatics.GetAllActorsOfClass` "/Game/Characters/Raphtalia_Root/BP_Raphtalia.BP_Raphtalia_C"))
  (for _array_element _outactors
    (bind _outactors_2 (`GameplayStatics.GetAllActorsOfClass` "/Game/Characters/Raphtalia_Root/BP_Raphtalia.BP_Raphtalia_C"))
    (for _array_element_2 _outactors_2
      (bind _returnvalue (`KismetMathLibrary.Vector_Distance` (`self.K2_GetActorLocation` _array_element_2) (`self.K2_GetActorLocation` _array_element)))
      (if (> _returnvalue (`self.ActualPlayersDistance`))
        (set `self.ActualPlayersDistance` _returnvalue)))))

(event `ReZoomCamera`
  (if (!= (`self.InitPlayersDistance`) 0.0)
    (`self.GetMaxPlayersDistance`)
    (set `SpringArmComponent.TargetArmLength` (`KismetMathLibrary.FClamp` (* (`self.InitArmLength`) (/ (`self.ActualPlayersDistance`) (`self.InitPlayersDistance`))) (`self.MinArmLength`) (`self.MaxArmLength`)) (`self.SpringArm`))))

(fn `UserConstructionScript`)