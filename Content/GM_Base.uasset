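; Base game mode for last-character-standing multiplayer rounds, tracking alive and dead PBCharacters.
; On match start it gathers all characters; each reported death updates the lists and checks whether one or none remains.
; It then increments survivors' GamesWon in the TestSlot save, matching players by unique net ID.
; Finally it shows the round winners widget and, after a delay, issues a non-seamless ServerTravel command targeting DesertPlayGround.
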(event `self.ReceiveBeginPlay`
  (add `self.OnMatchStarted` (delegate `GetCurrentPlayers`)))

(event `GetCurrentPlayers`
  (bind _outactors (`GameplayStatics.GetAllActorsOfClass` "/Script/ProjectB.PBCharacter"))
  (set `self.AliveCharacters` _outactors))

(event `PlayerDeath`
  (params (Character :type "PBCharacter Object Reference"))
  (`KismetArrayLibrary.Array_RemoveItem` (`self.AliveCharacters`) Character)
  (`KismetArrayLibrary.Array_AddUnique` (`self.DeathCharacters`) Character)
  (`self.CheckWinCon`))

(event `CheckWinCon`
  (if (<= (`KismetArrayLibrary.Array_Length` (`self.AliveCharacters`)) 1)
    (`self.GivePointsToPlayers`)))

(event `GivePointsToPlayers`
  (bind _returnvalue (`GameplayStatics.LoadGameFromSlot` "TestSlot"))
  (bind _assg_players_info (cast `/Game/SaveGame/SG_PlayersInfo` _returnvalue)
    (:`then`
      (set `self.PlayersInfo` _assg_players_info)
      (for _array_element (`self.AliveCharacters`)
        (for _array_element_2 (`/Game/SaveGame/SG_PlayersInfo.PlayersInfo` (`self.PlayersInfo`))
          (bind (_uid _gameswon) (break `/Game/SaveGame/PlayerSaveInfo` _array_element_2))
          (if (== (`GameplayStatics.GetPlayerStateFromUniqueNetId` _uid) (`Pawn.PlayerState` _array_element))
            (setmembers `/Game/SaveGame/PlayerSaveInfo` :`StructRef` _array_element_2 :`GamesWon` (+ _gameswon 1))
            (break))))
      (`GameplayStatics.SaveGameToSlot` (`self.PlayersInfo`) "TestSlot"))
    (:`CastFailed`
      _))
  (`self.MatchFinished`))

(event `MatchFinished`
  (`|CreateWidget` "/Game/Widgets/WBP_RoundWinners.WBP_RoundWinners_C")
  (`KismetSystemLibrary.Delay` 4.0)
  (`self.TravelToNextMap`))

(event `TravelToNextMap`
  (set `self.bUseSeamlessTravel` false)
  (`KismetSystemLibrary.ExecuteConsoleCommand` (`KismetStringLibrary.Concat_StrStr` "ServerTravel " "DesertPlayGround" "?Listen") null))

(fn `UserConstructionScript`)