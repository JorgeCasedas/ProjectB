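; BP_Nail is an ability projectile that flies along its own right vector and sticks to what it hits.
; On the server, overlapping any actor except the owner character stops movement, snap-attaches the nail to that actor's origin, reveals its widget and fires OnActorCollided.
; It exposes the attached actor through a getter and provides a DestroyNail event for removal.
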(event `self.ReceiveBeginPlay`
  (set `MovementComponent.Velocity` (* (`KismetMathLibrary.Normal` (`self.GetActorRightVector`)) (`self.Speed`)) (`self.ProjectileMovement`))
  (`SceneComponent.SetVisibility` (`self.Widget`) false false)
  (set `self.bIsAttached` false))

(event `self.Cube.OnComponentBeginOverlap`
  (params (OverlappedComponent :type "PrimitiveComponent Object Reference") (OtherActor :type "Actor Object Reference") (OtherComp :type "PrimitiveComponent Object Reference") (OtherBodyIndex :type Integer) (bFromSweep :type Boolean) (SweepResult :type "HitResult Structure (by ref)"))
  (if (and (`KismetSystemLibrary.IsServer`) (!= OtherActor (`self.OwnerCharacter`)))
    (`self.StopProjectile`)
    (bind _output_get (set `self.AttachedActor` OtherActor))
    (`self.K2_AttachToActor` _output_get "None" "SnapToTarget" "SnapToTarget" "KeepWorld")
    (set `self.bIsAttached` true)
    (`SceneComponent.SetVisibility` (`self.Widget`) true false)
    (`self.OnActorCollided`)))

(event `StopProjectile`
  (bind _projectilemovement (`self.ProjectileMovement`))
  (set `ProjectileMovementComponent.bSimulationEnabled` false _projectilemovement)
  (`ActorComponent.SetComponentTickEnabled` _projectilemovement false)
  (set `MovementComponent.Velocity` (0.0 0.0 0.0) (`self.ProjectileMovement`))
  (`PrimitiveComponent.SetSimulatePhysics` (`self.Cube`) false))

(event `DestroyNail`
  (`self.K2_DestroyActor`))

(fn `GetAttachedActor`
  (returns (AttachedActor :type "Actor Object Reference"))
  (return (`self.AttachedActor`)))

(fn `UserConstructionScript`)