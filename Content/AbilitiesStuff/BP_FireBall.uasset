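; BP_FireBall is a server-driven fireball projectile that applies a gameplay effect and a push to what it hits.
; On BeginPlay, the server launches it along the actor's right vector at Speed.
; When the Cube overlaps anything but the owner character, the server applies GE_Fireball if the target has an ability system, sends a push message from the fireball's location, then destroys the projectile.
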(event `self.ReceiveBeginPlay`
  (if (`KismetSystemLibrary.IsServer`)
    (set `MovementComponent.Velocity` (* (`KismetMathLibrary.Normal` (`self.GetActorRightVector`)) (`self.Speed`)) (`self.ProjectileMovement`))))

(event `self.Cube.OnComponentBeginOverlap`
  (params (OverlappedComponent :type "PrimitiveComponent Object Reference") (OtherActor :type "Actor Object Reference") (OtherComp :type "PrimitiveComponent Object Reference") (OtherBodyIndex :type Integer) (bFromSweep :type Boolean) (SweepResult :type "HitResult Structure (by ref)"))
  (bind _returnvalue (`AbilitySystemBlueprintLibrary.GetAbilitySystemComponent` OtherActor))
  (if (and (`KismetSystemLibrary.IsServer`) (!= OtherActor (`self.OwnerCharacter`)))
    (`/Engine/EditorBlueprintResources/StandardMacros.IsValid` _returnvalue
      (:`Is Valid`
        (`AbilitySystemComponent.BP_ApplyGameplayEffectToTarget` :`self` (`self.AbilitySystem`) :`GameplayEffectClass` "/Game/GAS/Effects/GE_Fireball.GE_Fireball_C" :`Target` _returnvalue))
      (:`Is Not Valid`
        _))
    (message `/Game/BPI_Pushable.PushActor` OtherActor (`self.K2_GetActorLocation`) 130.0)
    (`self.K2_DestroyActor`)))

(fn `GetAttachedActor`
  (returns (AttachedActor :type "Actor Object Reference"))
  (return (`self.AttachedActor`)))

(fn `UserConstructionScript`)