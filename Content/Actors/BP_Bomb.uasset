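; Hot-potato bomb that follows a random BP_Cat player from match start and passes to any non-owning cat that overlaps it.
; In team modes, it spawns BP_BombChild copies over the holder's teammates.
; The server handles ownership and the fuse timer, with a local countdown fallback for the camera-facing text.
; On expiry it activates GA_Bomb, plays explosion VFX on all bombs, then calls OnExploded.
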(event `ExplosionVFX`
  (`GameplayStatics.SpawnEmitterAtLocation` "/Game/FXVarietyPack/Particles/P_ky_explosion.P_ky_explosion" (`self.K2_GetActorLocation`) (struct) (2.0 2.0 2.0))
  (`self.SetActorHiddenInGame` true))

(event `self.ReceiveBeginPlay`
  (if (`KismetSystemLibrary.IsServer`)
    (bind _aspbgame_mode (cast `PBGameMode` (`GameplayStatics.GetGameMode`)))
    (bind _currentgamemodesettings_gamemode (break `GameModeSettings` (`PBGameMode.CurrentGameModeSettings` _aspbgame_mode)))
    (set `self.IsTeamsMode` (not (`|EnumEquality` _currentgamemodesettings_gamemode "AllVsAll")))
    (`self.SetActorHiddenInGame` true)
    (add `PBGameMode.OnMatchStarted` _aspbgame_mode (delegate `InitBomb`))))

(event `InitBomb`
  (bind _aspbplayer_state (cast `PBPlayerState` (`KismetArrayLibrary.Array_Random` (`GameStateBase.PlayerArray` (`GameplayStatics.GetGameState`)))))
  (`self.SetBombOwner` _aspbplayer_state)
  (`self.SetActorHiddenInGame` false)
  (bind _returnvalue (`KismetSystemLibrary.K2_SetTimerDelegate` (delegate `Explosion`) (`self.ExplosionTime`)))
  (set `self.ExplosionTimerHandle` _returnvalue)
  (`self.EnableBomb`))

(event `Explosion`
  (bind _abilitysystem (`self.AbilitySystem`))
  (`AbilitySystemComponent.K2_GiveAbility` _abilitysystem "/Game/GAS/Abilities/GA_Bomb.GA_Bomb_C" 0 -1)
  (`AbilitySystemComponent.TryActivateAbilityByClass` _abilitysystem "/Game/GAS/Abilities/GA_Bomb.GA_Bomb_C" true)
  (`self.ExplosionVFX`)
  (for _array_element (`self.SpawnedBombs`)
    (`/Game/Actors/BP_BombChild.ChildExplosionVFX` _array_element))
  (`KismetSystemLibrary.Delay` 1.0)
  (`self.OnExploded`))

(event `self.ReceiveTick`
  (params (DeltaSeconds :type "Float (single-precision)"))
  (bind _staticmesh (`self.StaticMesh`))
  (bind _output (`|GetArrayItem` (`self.CurrentOwner`)))
  (bind (_returnvalue_roll _returnvalue_pitch _returnvalue_yaw) (`KismetMathLibrary.BreakRotator` (`KismetMathLibrary.FindLookAtRotation` (`SceneComponent.K2_GetComponentLocation` (`self.TextRender`)) (`SceneComponent.K2_GetComponentLocation` (`PBLevelCamera.Camera` (`self.LevelCamera`))))))
  (`|ExecutionSequence`
    (:`then_0`
      (`SceneComponent.K2_AddLocalOffset` _staticmesh (* (`KismetMathLibrary.MakeVector` 0.0 0.0 (* (`KismetMathLibrary.Cos` (`KismetSystemLibrary.GetGameTimeInSeconds`)) -50.0)) (* DeltaSeconds (`self.HoverSpeed`))) false true)
      (`SceneComponent.K2_AddLocalRotation` _staticmesh (struct :`Yaw` 1.0) false false))
    (:`then_1`
      (`/Engine/EditorBlueprintResources/StandardMacros.IsValid` _output
        (:`Is Valid`
          (`self.K2_SetActorLocation` (`SceneComponent.K2_GetComponentLocation` (`/Game/Characters/Cat/BP_Cat.BombOffset` _output)))
          (for (_array_element _array_index) (`self.SpawnedBombs`)
            (bind _output_2 (`|GetArrayItem` (`self.CurrentOwner`) (+ _array_index 1)))
            (`/Engine/EditorBlueprintResources/StandardMacros.IsValid` _output_2
              (:`Is Valid`
                (`self.K2_SetActorLocation` _array_element (`SceneComponent.K2_GetComponentLocation` (`/Game/Characters/Cat/BP_Cat.BombOffset` _output_2)) false false)))))))
    (:`then_2`
      (if (`self.bIsBombEnabled`)
        (`/Engine/EditorBlueprintResources/StandardMacros.IsValid` (`self.LevelCamera`)
          (:`Is Valid`
            _)
          (:`Is Not Valid`
            (bind _returnvalue (`GameplayStatics.GetActorOfClass` "/Game/Cameras/BP_LevelCamera.BP_LevelCamera_C"))
            (set `self.LevelCamera` _returnvalue)))
        (`SceneComponent.K2_SetWorldRotation` (`self.TextRender`) (`KismetMathLibrary.MakeRotator` _returnvalue_roll _returnvalue_pitch _returnvalue_yaw) false false)
        (if (`KismetSystemLibrary.K2_IsValidTimerHandle` (`self.ExplosionTimerHandle`))
          (`TextRenderComponent.K2_SetText` (`self.TextRender`) (`KismetTextLibrary.Conv_Int64ToText` (`KismetMathLibrary.FFloor64` (`KismetSystemLibrary.K2_GetTimerRemainingTimeHandle` (`self.ExplosionTimerHandle`)))))
          (else
            (set `self.ExplosionTime` (- (`self.ExplosionTime`) (`GameplayStatics.GetWorldDeltaSeconds`)))
            (`TextRenderComponent.K2_SetText` (`self.TextRender`) (`KismetTextLibrary.Conv_Int64ToText` (`KismetMathLibrary.FFloor64` (`KismetMathLibrary.FClamp` (`self.ExplosionTime`) 0.0 10000.0))))))))))

(event `EnableBomb`
  (set `self.bIsBombEnabled` true))

(event `self.Capsule.OnComponentBeginOverlap`
  (params (OverlappedComponent :type "PrimitiveComponent Object Reference") (OtherActor :type "Actor Object Reference") (OtherComp :type "PrimitiveComponent Object Reference") (OtherBodyIndex :type Integer) (bFromSweep :type Boolean) (SweepResult :type "HitResult Structure (by ref)"))
  (`self.BombChildOverlappedWithActor` OtherActor))

(event `BombChildOverlappedWithActor`
  (params (Actor :type "Actor Object Reference"))
  (if (`KismetSystemLibrary.IsServer`)
    (bind _asbp_cat (cast `/Game/Characters/Cat/BP_Cat` Actor))
    (if (< (`KismetArrayLibrary.Array_Find` (`self.CurrentOwner`) _asbp_cat) 0)
      (bind _aspbplayer_state (cast `PBPlayerState` (`Pawn.PlayerState` _asbp_cat)))
      (`self.SetBombOwner` _aspbplayer_state))))

(fn `SetBombOwner`
  (params (OwnerState :type "PBPlayerState Object Reference"))
  (for _array_element (`self.SpawnedBombs`)
    (`self.K2_DestroyActor` _array_element))
  (`KismetArrayLibrary.Array_Clear` (`self.CurrentOwner`))
  (`KismetArrayLibrary.Array_Clear` (`self.SpawnedBombs`))
  (bind _asbp_cat (cast `/Game/Characters/Cat/BP_Cat` (`PlayerState.GetPawn` (`local.OwnerState`))))
  (`KismetArrayLibrary.Array_AddUnique` (`self.CurrentOwner`) _asbp_cat)
  (if (`self.IsTeamsMode`)
    (bind _returnvalue (`PBPlayerState.GetTeamID` (`local.OwnerState`)))
    (bind _aspbgame_mode (cast `PBGameMode` (`GameplayStatics.GetGameMode`)))
    (for _array_element_2 (`PBGameMode.PlayersByTeams` _aspbgame_mode)
      (bind (_teamid _players) (break `PlayersByTeam` _array_element_2))
      (if (== _teamid _returnvalue)
        (for _array_element_3 _players
          (bind _asbp_cat_2 (cast `/Game/Characters/Cat/BP_Cat` (`PlayerState.GetPawn` _array_element_3)))
          (bind _returnvalue_2 (`KismetArrayLibrary.Array_AddUnique` (`self.CurrentOwner`) _asbp_cat_2))
          (if (> _returnvalue_2 -1)
            (bind _returnvalue_3 (`|SpawnActorFromClass` "/Game/Actors/BP_BombChild.BP_BombChild_C" (`KismetMathLibrary.MakeTransform` (0.0 0.0 0.0)) "Undefined" "MultiplyWithRoot" null self null))
            (`KismetArrayLibrary.Array_AddUnique` (`self.SpawnedBombs`) _returnvalue_3)))))))

(fn `UserConstructionScript`)