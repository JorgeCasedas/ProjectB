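; BP_BombChild is a child bomb actor that reports its capsule overlaps to its BombFather, which handles the response.
; Each tick it spins its mesh, mirrors the father's text label and turns that label toward a cached BP_LevelCamera.
; A cosine hover offset is present but multiplied by zero, so the mesh does not bob.
; ChildExplosionVFX spawns an explosion emitter and hides the actor without destroying it.
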(event `ChildExplosionVFX`
  (`GameplayStatics.SpawnEmitterAtLocation` "/Game/FXVarietyPack/Particles/P_ky_explosion.P_ky_explosion" (`self.K2_GetActorLocation`) (struct) (2.0 2.0 2.0))
  (`self.SetActorHiddenInGame` true))

(event `self.ReceiveTick`
  (params (DeltaSeconds :type "Float (single-precision)"))
  (bind _staticmesh (`self.StaticMesh`))
  (bind (_returnvalue_roll _returnvalue_pitch _returnvalue_yaw) (`KismetMathLibrary.BreakRotator` (`KismetMathLibrary.FindLookAtRotation` (`SceneComponent.K2_GetComponentLocation` (`self.TextRender`)) (`SceneComponent.K2_GetComponentLocation` (`PBLevelCamera.Camera` (`self.LevelCamera`))))))
  (`|ExecutionSequence`
    (:`then_0`
      (`SceneComponent.K2_AddLocalOffset` _staticmesh (* (`KismetMathLibrary.MakeVector` 0.0 0.0 (* (`KismetMathLibrary.Cos` (`KismetSystemLibrary.GetGameTimeInSeconds`)) -50.0)) (* 0.0 (`self.HoverSpeed`))) false true)
      (`SceneComponent.K2_AddLocalRotation` _staticmesh (struct :`Yaw` 1.0) false false))
    (:`then_1`
      (`TextRenderComponent.K2_SetText` (`self.TextRender`) (`TextRenderComponent.Text` (`/Game/Actors/BP_Bomb.TextRender` (`self.BombFather`))))
      (`/Engine/EditorBlueprintResources/StandardMacros.IsValid` (`self.LevelCamera`)
        (:`Is Valid`
          _)
        (:`Is Not Valid`
          (bind _returnvalue (`GameplayStatics.GetActorOfClass` "/Game/Cameras/BP_LevelCamera.BP_LevelCamera_C"))
          (set `self.LevelCamera` _returnvalue)))
      (`SceneComponent.K2_SetWorldRotation` (`self.TextRender`) (`KismetMathLibrary.MakeRotator` _returnvalue_roll _returnvalue_pitch _returnvalue_yaw) false false))))

(event `self.Capsule.OnComponentBeginOverlap`
  (params (OverlappedComponent :type "PrimitiveComponent Object Reference") (OtherActor :type "Actor Object Reference") (OtherComp :type "PrimitiveComponent Object Reference") (OtherBodyIndex :type Integer) (bFromSweep :type Boolean) (SweepResult :type "HitResult Structure (by ref)"))
  (bind _bombfather (`self.BombFather`))
  (`/Engine/EditorBlueprintResources/StandardMacros.IsValid` _bombfather
    (:`Is Valid`
      (`/Game/Actors/BP_Bomb.BombChildOverlappedWithActor` _bombfather OtherActor))))

(fn `UserConstructionScript`)