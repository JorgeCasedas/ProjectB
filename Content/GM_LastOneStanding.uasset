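; Game mode for Last One Standing that handles player ability saving and selection, with notes marking logic to move to C++ or a base game mode.
; MatchStarted initializes the save through the game instance, then writes each player state's gameplay abilities to the hardcoded TestSlot.
; CharacterSelectedAbility grants the indexed ability from a per-controller map to that player's BP_Cat with an input tag.
; The login chain filling that map and the match-start binding are disconnected.
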(event `MatchStarted`
  ;[1 0 0] Move to c++
  (bind _asproject_bgame_instance (cast `ProjectBGameInstance` (`GameplayStatics.GetGameInstance`)))
  (`ProjectBGameInstance.SetInitialSaveGame` _asproject_bgame_instance)
  (bind _returnvalue (`GameplayStatics.LoadGameFromSlot` "TestSlot"))
  (bind _assave_game_player_info (cast `SaveGamePlayerInfo` _returnvalue))
  (set `self.TestSaveGame` _assave_game_player_info)
  (for _array_element (`GameStateBase.PlayerArray` (`GameplayStatics.GetGameState`))
    (bind _aspbplayer_state (cast `PBPlayerState` _array_element))
    (`SaveGamePlayerInfo.SaveGameplayAbilities` (`self.TestSaveGame`) _aspbplayer_state))
  (`GameplayStatics.SaveGameToSlot` (`self.TestSaveGame`) "TestSlot"))

(event `CharacterSelectedAbility`
  (params (SelectedAbilityIndex :type Integer) (GameplayTag :type "GameplayTag Structure") (PlayerController :type "PlayerController Object Reference"))
  ;[1 0 0] This should be in the base game mode
  (bind _keys (`BlueprintMapLibrary.Map_Keys` (`self.TempAbilitiesGivenToPlayers`)))
  (for _array_element _keys
    (if (== PlayerController _array_element)
      (for (_array_element_2 _array_index) (`.Abilities` (break `GameplayAbilitiesArray` (`BlueprintMapLibrary.Map_Find` (`self.TempAbilitiesGivenToPlayers`) _array_element)))
        (if (== _array_index SelectedAbilityIndex)
          (bind _aspbcharacter (cast `PBCharacter` (`Controller.K2_GetPawn` PlayerController)))
          (bind _asbp_cat (cast `/Game/Characters/Cat/BP_Cat` _aspbcharacter))
          (`/Game/Characters/Cat/BP_Cat.AddSelectedAbility` _asbp_cat _array_element_2 GameplayTag))))))

(fn `UserConstructionScript`)