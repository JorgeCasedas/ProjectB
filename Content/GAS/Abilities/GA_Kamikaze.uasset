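; GA_Kamikaze is a gameplay ability that makes its avatar explode after a delay, pushing and damaging nearby actors.
; Once committed, the server starts a timer that runs a sphere trace around the avatar, ignoring the avatar itself.
; Each unique hit receives a push message from the blast origin, plus GE_ExplosionDamage if it has an ability system component.
; A tick later, a BP_Cat avatar takes the same damage effect and the ability ends.
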(event `self.K2_ActivateAbility`
  (bind _returnvalue (`self.K2_CommitAbility`))
  (if _returnvalue
    (if (`KismetSystemLibrary.IsServer`)
      (`KismetSystemLibrary.K2_SetTimerDelegate` (delegate `Explosion`) (`self.ExplosionDelay`)))))

(event `Explosion`
  (bind _returnvalue (`self.GetAvatarActorFromActorInfo`))
  (bind _actorshit (`self.ActorsHit`))
  (bind _returnvalue_2 (`Actor.K2_GetActorLocation` _returnvalue))
  (bind _outhits (`KismetSystemLibrary.SphereTraceMultiForObjects` _returnvalue_2 _returnvalue_2 (`self.ExplosionRadius`) (`|MakeArray` "ObjectTypeQuery2" "ObjectTypeQuery3" "ObjectTypeQuery4" :!type "EObjectTypeQuery Enum") false (`|MakeArray` _returnvalue)))
  (for _array_element _outhits
    (bind (_bblockinghit _binitialoverlap _time _distance _location _impactpoint _normal _impactnormal _physmat _hitactor) (`GameplayStatics.BreakHitResult` _array_element))
    (if (< (`KismetArrayLibrary.Array_Find` _actorshit _hitactor) 0)
      (`KismetArrayLibrary.Array_AddUnique` _actorshit _hitactor)
      (message `/Game/BPI_Pushable.PushActor` _hitactor (`Actor.K2_GetActorLocation` (`self.GetAvatarActorFromActorInfo`)) (`self.ExplosionForce`))
      (`/Engine/EditorBlueprintResources/StandardMacros.IsValid` (`AbilitySystemBlueprintLibrary.GetAbilitySystemComponent` _hitactor)
        (:`Is Valid`
          (`self.BP_ApplyGameplayEffectToTarget` (`AbilitySystemBlueprintLibrary.AbilityTargetDataFromActor` _hitactor) "/Game/GAS/Effects/GE_ExplosionDamage.GE_ExplosionDamage_C")))))
  (`KismetSystemLibrary.DelayUntilNextTick`)
  (cast `/Game/Characters/Cat/BP_Cat` (`self.GetAvatarActorFromActorInfo`)
    (:`then`
      (`self.BP_ApplyGameplayEffectToOwner` "/Game/GAS/Effects/GE_ExplosionDamage.GE_ExplosionDamage_C"))
    (:`CastFailed`
      _))
  (`self.K2_EndAbility`))