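; GAS ability for the cat's jump attack: a forward lunge in flying mode that finishes with a punch.
; Activation disables input and mouse-facing, launches the cat and plays the flying montage, until a JumpAttack gameplay event or a one-second timeout stops it.
; StopJump restores walking and plays a sped-up punch montage, applying GE_Punch to targets from a Damage event.
; Montage end ends the ability, restoring input and mouse-facing.
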(event `self.K2_ActivateAbility`
  (bind _returnvalue (`self.K2_CommitAbility`))
  (if _returnvalue
    (bind _asbp_cat (cast `/Game/Characters/Cat/BP_Cat` (`self.GetAvatarActorFromActorInfo`)))
    (`/Game/Characters/Cat/BP_Cat.HandleJumpAttack` _asbp_cat true)
    (set `PBCharacter.bLookTowardsMouse` false _asbp_cat)
    (bind _charactermovement (`Character.CharacterMovement` _asbp_cat))
    (`CharacterMovementComponent.SetMovementMode` _charactermovement "MOVE_Flying" 0)
    (bind _asplayer_controller (cast `PlayerController` (`Pawn.GetController` _asbp_cat)))
    (`Actor.DisableInput` _asplayer_controller null)
    (set `MovementComponent.Velocity` (* (`KismetMathLibrary.Normal` (`Actor.GetActorForwardVector` _asbp_cat)) 3000.0) _charactermovement)
    (`AbilityTask_PlayMontageAndWait.CreatePlayMontageAndWaitProxy` "None" "/Game/Characters/Cat/Animations/Flying_Montage.Flying_Montage" 1.0 "None" false
      (:`then`
        (bind _asynctaskproxy (`AbilityTask_WaitGameplayEvent.WaitGameplayEvent` (struct :`TagName` "Ability.Active.JumpAttack") null true)
          (:`then`
            (set `self.WaitStopEvent` _asynctaskproxy)
            (`KismetSystemLibrary.Delay` 1.0))
          (:`EventReceived`
            _))
        (`/Engine/EditorBlueprintResources/StandardMacros.IsValid` (`self.WaitStopEvent`)
          (:`Is Valid`
            (`GameplayTask.EndTask` (`self.WaitStopEvent`))
            (set `self.WaitStopEvent` null)
            (`self.StopJump`)))))))

(event `StopJump`
  (bind _asbp_cat (cast `/Game/Characters/Cat/BP_Cat` (`self.GetAvatarActorFromActorInfo`)))
  (`/Game/Characters/Cat/BP_Cat.HandleJumpAttack` _asbp_cat false)
  (bind _charactermovement (`Character.CharacterMovement` _asbp_cat))
  (`CharacterMovementComponent.SetMovementMode` _charactermovement "MOVE_Walking" 0)
  (set `MovementComponent.Velocity` (0.0 0.0 0.0) _charactermovement)
  (`KismetSystemLibrary.PrintString` "StopJump")
  (`AbilityTask_PlayMontageAndWait.CreatePlayMontageAndWaitProxy` "None" "/Game/Characters/Cat/Animations/CatPunch_Montage.CatPunch_Montage" 3.0
    (:`then`
      (bind (_asynctaskproxy _payload) (`AbilityTask_WaitGameplayEvent.WaitGameplayEvent` (struct :`TagName` "Ability.Damage") null)
        (:`then`
          (set `self.WaitEventTask` _asynctaskproxy))
        (:`EventReceived`
          (`self.BP_ApplyGameplayEffectToTarget` (`.TargetData` (break `GameplayEventData` _payload)) "/Game/GAS/Effects/GE_Punch.GE_Punch_C")
          (`GameplayTask.EndTask` (`self.WaitEventTask`)))))
    (:`OnCompleted`
      (`self.K2_EndAbility` :!label _label))
    (:`OnBlendOut`
      (goto _label))
    (:`OnInterrupted`
      (goto _label))
    (:`OnCancelled`
      (goto _label))))

(event `self.K2_OnEndAbility`
  (params (bWasCancelled :type Boolean))
  (bind _asbp_cat (cast `/Game/Characters/Cat/BP_Cat` (`self.GetAvatarActorFromActorInfo`)))
  (bind _asplayer_controller (cast `PlayerController` (`Pawn.GetController` _asbp_cat)))
  (`Actor.EnableInput` _asplayer_controller null)
  (set `PBCharacter.bLookTowardsMouse` true _asbp_cat)
  (`GameplayTask.EndTask` (`self.WaitEventTask`)))