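; GA_Meow is a Gameplay Ability that sets off a radial push around its avatar, knocking away nearby actors.
; On the server, it commits, then sphere-traces at the avatar's location for WorldDynamic, Pawn and PhysicsBody objects, with timed debug drawing.
; Each unique hit actor, excluding the avatar, receives PushActorMessage with the avatar's location and ExplosionForce.
; EndAbility runs only after a successful server commit.
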(event `self.K2_ActivateAbility`
  (bind _returnvalue (`self.GetAvatarActorFromActorInfo`))
  (bind _actorshit (`self.ActorsHit`))
  (bind _returnvalue_2 (`Actor.K2_GetActorLocation` _returnvalue))
  (if (`KismetSystemLibrary.IsServer`)
    (bind _returnvalue_3 (`self.K2_CommitAbility`))
    (if _returnvalue_3
      (`KismetArrayLibrary.Array_Clear` (`self.ActorsHit`))
      (bind _outhits (`KismetSystemLibrary.SphereTraceMultiForObjects` _returnvalue_2 _returnvalue_2 (`self.ExplosionRadius`) (`|MakeArray` "ObjectTypeQuery2" "ObjectTypeQuery3" "ObjectTypeQuery4" :!type "EObjectTypeQuery Enum") false (`|MakeArray` _returnvalue) "ForDuration" true (struct :`R` 1.0 :`A` 1.0) (struct :`G` 1.0 :`A` 1.0) 0.5))
      (for _array_element _outhits
        (bind (_bblockinghit _binitialoverlap _time _distance _location _impactpoint _normal _impactnormal _physmat _hitactor) (`GameplayStatics.BreakHitResult` _array_element))
        (if (< (`KismetArrayLibrary.Array_Find` _actorshit _hitactor) 0)
          (`KismetArrayLibrary.Array_AddUnique` _actorshit _hitactor)
          (message `/Game/BPI_Pushable.PushActor` _hitactor (`Actor.K2_GetActorLocation` (`self.GetAvatarActorFromActorInfo`)) (`self.ExplosionForce`))))
      (`self.K2_EndAbility`))))