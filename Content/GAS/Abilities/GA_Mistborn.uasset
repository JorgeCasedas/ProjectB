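; Mistborn gameplay ability for BP_Cat that spawns a nail and, on a second press once it attaches, pulls along the line to it.
; Comparing both weight values decides whether the cat, the attached actor or both move, using per-tick velocity with Flying mode or disabled gravity.
; A NailReached gameplay event stops the pull and commits cooldown.
; Separate flight and attachment timers handle timeouts, and ending destroys the nail.
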(event `self.K2_ActivateAbility`
  (bind _playerpawn (`self.PlayerPawn`))
  (bind _flyingtimeout (`self.FlyingTimeOut`))
  (bind _asbp_cat (cast `/Game/Characters/Cat/BP_Cat` (`self.GetAvatarActorFromActorInfo`)))
  (set `self.PlayerPawn` _asbp_cat)
  (bind _returnvalue (`|SpawnActorFromClass` "/Game/AbilitiesStuff/BP_Nail.BP_Nail_C" (`KismetMathLibrary.MakeTransform` (`Actor.K2_GetActorLocation` _playerpawn) (`SceneComponent.K2_GetComponentRotation` (`Character.Mesh` _playerpawn))) "Undefined" "MultiplyWithRoot" null 1000.0 _playerpawn null))
  (bind _output_get (set `self.SpawnedNail` _returnvalue))
  (add `/Game/AbilitiesStuff/BP_Nail.OnActorCollided` _output_get (`|CreateDelegate` :!event `OnNailAttached`))
  (`self.OnNailSpawned` _flyingtimeout (`Pawn.PlayerState` (`self.PlayerPawn`)))
  (bind _returnvalue_2 (`KismetSystemLibrary.K2_SetTimerDelegate` (`|CreateDelegate` :!event `AbilityTimeOut`) _flyingtimeout))
  (set `self.FlyingTimeOutTimer` _returnvalue_2)
  (bind _asynctaskproxy (`AbilityTask_WaitInputPress.WaitInputPress` false :!label _label)
    (:`then`
      (set `self.WaitInputPress` _asynctaskproxy))
    (:`OnPress`
      (if (`/Game/AbilitiesStuff/BP_Nail.bIsAttached` (`self.SpawnedNail`))
        (`self.Reactivation`)
        (else
          (goto _label))))))

(event `OnNailAttached`
  (params (Owner :type "/Game/Characters/Cat/BP_Cat Object Reference"))
  (`KismetSystemLibrary.K2_ClearAndInvalidateTimerHandle` (`self.FlyingTimeOutTimer`))
  (bind _returnvalue (`KismetSystemLibrary.K2_SetTimerDelegate` (`|CreateDelegate` :!event `AbilityTimeOut`) (`self.AttachedTimeOut`)))
  (set `self.AttachedTimeOutTimer` _returnvalue)
  (`self.OnNailReached` (`Pawn.PlayerState` Owner)))

(event `OnNailAttachedClient`
  (params (Owner :type "/Game/Characters/Cat/BP_Cat Object Reference")))

(event `AbilityTimeOut`
  (set `self.ShouldCommitCooldown` false)
  (`self.K2_EndAbility`))

(event `Reactivation`
  (bind _playerpawn (`self.PlayerPawn`))
  (`KismetSystemLibrary.PrintString` "Pull")
  (bind _newparam (message `/Game/BPI_ActorWeight.GetWeight` (`self.PlayerPawn`)))
  (bind _attachedactor (`/Game/AbilitiesStuff/BP_Nail.GetAttachedActor` (`self.SpawnedNail`)))
  (bind _newparam_2 (message `/Game/BPI_ActorWeight.GetWeight` _attachedactor))
  (`/Engine/EditorBlueprintResources/StandardMacros.CompareInt` (`KismetMathLibrary.Conv_ByteToInt` _newparam) (`KismetMathLibrary.Conv_ByteToInt` _newparam_2)
    (:`>`
      (`Actor.DisableInput` _playerpawn (cast `PlayerController` (`Pawn.GetController` _playerpawn) :!pure true) :!label _label_2)
      (`CharacterMovementComponent.SetMovementMode` (`Character.CharacterMovement` (`self.PlayerPawn`)) "MOVE_Flying" 0)
      (`self.SetPlayerVelocity`))
    (:`==`
      (`|ExecutionSequence`
        (:`then_0`
          (goto _label_2))
        (:`then_1`
          (bind _attachedactor_2 (`/Game/AbilitiesStuff/BP_Nail.GetAttachedActor` (`self.SpawnedNail`) :!label _label_3))
          (`self.SetActorMovement` _attachedactor_2 true))))
    (:`<`
      (goto _label_3)))
  (`/Game/Characters/Cat/BP_Cat.HandleMistborn` (`self.PlayerPawn`) (`self.SpawnedNail`))
  (`/Engine/EditorBlueprintResources/StandardMacros.IsValid` (`self.NailReachedAsync`)
    (:`Is Not Valid`
      (bind _asynctaskproxy (`AbilityTask_WaitGameplayEvent.WaitGameplayEvent` (struct :`TagName` "Ability.Active.Mistborn.NailReached") null true)
        (:`then`
          (set `self.NailReachedAsync` _asynctaskproxy)
          (`KismetSystemLibrary.K2_ClearAndInvalidateTimerHandle` (`self.AttachedTimeOutTimer`)))
        (:`EventReceived`
          (`self.StopPull`))))))

(event `SetPlayerVelocity`
  (bind _charactermovement (`Character.CharacterMovement` (`self.PlayerPawn`)))
  (if (`|EnumEquality` (`CharacterMovementComponent.MovementMode` _charactermovement) "MOVE_Flying")
    (set `MovementComponent.Velocity` (* (`KismetMathLibrary.Normal` (- (`Actor.K2_GetActorLocation` (`self.SpawnedNail`)) (`Actor.K2_GetActorLocation` (`self.PlayerPawn`)))) (`self.PullSpeed`)) _charactermovement)
    (`KismetSystemLibrary.DelayUntilNextTick`)
    (`self.SetPlayerVelocity`)))

(event `SetOtherPlayerVelocity`
  (params (Component :type "CharacterMovementComponent Object Reference"))
  (if (`|EnumEquality` (`CharacterMovementComponent.MovementMode` Component) "MOVE_Flying")
    (set `MovementComponent.Velocity` (* (`KismetMathLibrary.Normal` (- (`Actor.K2_GetActorLocation` (`self.PlayerPawn`)) (`Actor.K2_GetActorLocation` (`self.SpawnedNail`)))) (`self.PullSpeed`)) Component)
    (`KismetSystemLibrary.DelayUntilNextTick`)
    (`self.SetOtherPlayerVelocity` Component)
    (else
      (`MovementComponent.StopMovementImmediately` Component))))

(event `SetActorMovement`
  (params (Actor :type "Actor Object Reference") (Enabled :type Boolean))
  (bind _returnvalue (`Actor.GetComponentByClass` Actor "/Script/Engine.PrimitiveComponent"))
  (bind _returnvalue_2 (`Actor.GetComponentByClass` Actor "/Script/Engine.CharacterMovementComponent"))
  (`/Engine/EditorBlueprintResources/StandardMacros.IsValid` _returnvalue_2
    (:`Is Valid`
      (`CharacterMovementComponent.SetMovementMode` _returnvalue_2 (select `bool` Enabled :`false` "MOVE_Walking" :`true` "MOVE_Flying" :!type "EMovementMode Enum") 0)
      (`self.SetOtherPlayerVelocity` _returnvalue_2))
    (:`Is Not Valid`
      (`PrimitiveComponent.SetEnableGravity` _returnvalue (not Enabled))
      (`self.SetOtherActorVelocity` _returnvalue))))

(event `SetOtherActorVelocity`
  (params (Component :type "PrimitiveComponent Object Reference"))
  (if (`PrimitiveComponent.IsGravityEnabled` Component)
    (`PrimitiveComponent.SetPhysicsLinearVelocity` Component (0.0 0.0 0.0) false "None")
    (else
      (`PrimitiveComponent.SetPhysicsLinearVelocity` Component (* (`KismetMathLibrary.Normal` (- (`Actor.K2_GetActorLocation` (`self.PlayerPawn`)) (`Actor.K2_GetActorLocation` (`self.SpawnedNail`)))) (`self.PullSpeed`)) false "None")
      (`KismetSystemLibrary.DelayUntilNextTick`)
      (`self.SetOtherActorVelocity` Component))))

(event `StopPull`
  (bind _playerpawn (`self.PlayerPawn`))
  (bind _charactermovement (`Character.CharacterMovement` (`self.PlayerPawn`)))
  (`Actor.EnableInput` _playerpawn (cast `PlayerController` (`Pawn.GetController` _playerpawn) :!pure true))
  (`MovementComponent.StopMovementImmediately` _charactermovement)
  (`CharacterMovementComponent.SetMovementMode` _charactermovement "MOVE_Walking" 0)
  (`/Game/Characters/Cat/BP_Cat.HandleMistborn` (`self.PlayerPawn`) null)
  (bind _attachedactor (`/Game/AbilitiesStuff/BP_Nail.GetAttachedActor` (`self.SpawnedNail`)))
  (`self.SetActorMovement` _attachedactor)
  (set `self.ShouldCommitCooldown` true)
  (`self.K2_EndAbility`))

(event `self.K2_OnEndAbility`
  (params (bWasCancelled :type Boolean))
  (bind _waitinputpress (`self.WaitInputPress`))
  (`/Game/AbilitiesStuff/BP_Nail.DestroyNail` (`self.SpawnedNail`))
  (`KismetSystemLibrary.K2_ClearAndInvalidateTimerHandle` (`self.FlyingTimeOutTimer`))
  (`KismetSystemLibrary.K2_ClearAndInvalidateTimerHandle` (`self.AttachedTimeOutTimer`))
  (if (`self.ShouldCommitCooldown`)
    (`self.K2_CommitAbility`))
  (`/Engine/EditorBlueprintResources/StandardMacros.IsValid` _waitinputpress
    (:`Is Valid`
      (`GameplayTask.EndTask` _waitinputpress))))