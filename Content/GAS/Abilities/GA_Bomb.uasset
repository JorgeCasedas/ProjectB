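; GA_Bomb is a gameplay ability that makes a bomb explode, pushing nearby actors away and killing its owners.
; A sphere overlap trace at the avatar's location finds objects within the explosion radius and sends each unique actor a push message from that origin.
; One tick later, it applies GE_InstantDeath to each entry in BP_Bomb's CurrentOwner list, calling EndAbility inside that loop.
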(event `self.K2_ActivateAbility`
  (bind _returnvalue (`self.GetAvatarActorFromActorInfo`))
  (bind _actorshit (`self.ActorsHit`))
  (bind _returnvalue_2 (`Actor.K2_GetActorLocation` _returnvalue))
  (bind _outhits (`KismetSystemLibrary.SphereTraceMultiForObjects` _returnvalue_2 _returnvalue_2 (`self.ExplosionRadius`) (`|MakeArray` "ObjectTypeQuery2" "ObjectTypeQuery3" "ObjectTypeQuery4" :!type "EObjectTypeQuery Enum") false (`|MakeArray` _returnvalue)))
  (for _array_element _outhits
    (bind (_bblockinghit _binitialoverlap _time _distance _location _impactpoint _normal _impactnormal _physmat _hitactor) (`GameplayStatics.BreakHitResult` _array_element))
    (if (< (`KismetArrayLibrary.Array_Find` _actorshit _hitactor) 0)
      (`KismetArrayLibrary.Array_AddUnique` _actorshit _hitactor)
      (message `/Game/BPI_Pushable.PushActor` _hitactor (`Actor.K2_GetActorLocation` (`self.GetAvatarActorFromActorInfo`)) (`self.ExplosionForce`))))
  (`KismetSystemLibrary.DelayUntilNextTick`)
  (bind _asbp_bomb (cast `/Game/Actors/BP_Bomb` (`self.GetOwningActorFromActorInfo`)))
  (for _array_element_2 (`/Game/Actors/BP_Bomb.CurrentOwner` _asbp_bomb)
    (bind _returnvalue_3 (`AbilitySystemBlueprintLibrary.GetAbilitySystemComponent` _array_element_2))
    (`AbilitySystemComponent.BP_ApplyGameplayEffectToSelf` _returnvalue_3 "/Game/GAS/Effects/GE_InstantDeath.GE_InstantDeath_C" 0.0 (`AbilitySystemComponent.MakeEffectContext` _returnvalue_3))
    (`self.K2_EndAbility`)))