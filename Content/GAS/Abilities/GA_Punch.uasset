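; Gameplay ability that performs a punch for a player-controlled PBCharacter, applying damage through GAS.
; After committing, it disables the player's input and plays the sped-up CatPunch montage while waiting for an Ability.Damage gameplay event.
; That event's target data receives GE_Punch.
; Any montage exit ends the ability, which stops the stored wait task and restores input.
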(event `self.K2_ActivateAbility`
  (bind _returnvalue (`self.GetAvatarActorFromActorInfo`))
  (bind _returnvalue_2 (`self.K2_CommitAbility`))
  (if _returnvalue_2
    (bind _aspbcharacter (cast `PBCharacter` _returnvalue))
    (bind _asplayer_controller (cast `PlayerController` (`Pawn.GetController` _aspbcharacter)))
    (`/Engine/EditorBlueprintResources/StandardMacros.IsValid` _asplayer_controller
      (:`Is Valid`
        (`Actor.DisableInput` _returnvalue _asplayer_controller)
        (`AbilityTask_PlayMontageAndWait.CreatePlayMontageAndWaitProxy` "None" "/Game/Characters/Cat/Animations/CatPunch_Montage.CatPunch_Montage" 2.5
          (:`then`
            (bind (_asynctaskproxy _payload) (`AbilityTask_WaitGameplayEvent.WaitGameplayEvent` (struct :`TagName` "Ability.Damage") null)
              (:`then`
                (set `self.WaitEventTask` _asynctaskproxy))
              (:`EventReceived`
                (`self.BP_ApplyGameplayEffectToTarget` (`.TargetData` (break `GameplayEventData` _payload)) "/Game/GAS/Effects/GE_Punch.GE_Punch_C"))))
          (:`OnCompleted`
            (`self.K2_EndAbility` :!label _label))
          (:`OnBlendOut`
            (goto _label))
          (:`OnInterrupted`
            (goto _label))
          (:`OnCancelled`
            (goto _label)))))))

(event `self.K2_OnEndAbility`
  (params (bWasCancelled :type Boolean))
  (bind _returnvalue (`self.GetAvatarActorFromActorInfo`))
  (bind _waiteventtask (`self.WaitEventTask`))
  (`|ExecutionSequence`
    (:`then_0`
      (`/Engine/EditorBlueprintResources/StandardMacros.IsValid` _waiteventtask
        (:`Is Valid`
          (`GameplayTask.EndTask` _waiteventtask))))
    (:`then_1`
      (bind _aspbcharacter (cast `PBCharacter` _returnvalue))
      (bind _asplayer_controller (cast `PlayerController` (`Pawn.GetController` _aspbcharacter)))
      (`/Engine/EditorBlueprintResources/StandardMacros.IsValid` _asplayer_controller
        (:`Is Valid`
          (`Actor.EnableInput` _returnvalue _asplayer_controller))))))