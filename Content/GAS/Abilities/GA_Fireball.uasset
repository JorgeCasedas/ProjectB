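; Gameplay ability that spawns a BP_FireBall projectile from the BP_Cat avatar.
; On activation, only the server commits the ability, casts the avatar to BP_Cat and stores it as PlayerPawn.
; It spawns the fireball at the cat's location using its mesh's world rotation, passes the cat as OwnerCharacter, stores the reference and ends the ability.
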(event `self.K2_ActivateAbility`
  (bind _playerpawn (`self.PlayerPawn`))
  (if (`KismetSystemLibrary.IsServer`)
    (`self.K2_CommitAbility`)
    (bind _asbp_cat (cast `/Game/Characters/Cat/BP_Cat` (`self.GetAvatarActorFromActorInfo`)))
    (set `self.PlayerPawn` _asbp_cat)
    (bind _returnvalue (`|SpawnActorFromClass` "/Game/AbilitiesStuff/BP_FireBall.BP_FireBall_C" (`KismetMathLibrary.MakeTransform` (`Actor.K2_GetActorLocation` _playerpawn) (`SceneComponent.K2_GetComponentRotation` (`Character.Mesh` _playerpawn))) "Undefined" "MultiplyWithRoot" null 1000.0 _playerpawn null))
    (set `self.Fireball` _returnvalue)
    (`self.K2_EndAbility`)))