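; Base game mode that handles timed team swaps, win presentation and a count of connected players.
; It binds to match start, match end, player win and login events on BeginPlay.
; If the win-condition rules include ChangeTeamEveryXSeconds, a looping timer calls ChangePlayersTeams until the match ends.
; Winners are collected uniquely, and the first win arms a match-end handler that shows the game-won screen on every PC_Base controller.
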(event `self.ReceiveBeginPlay`
  (`parent.ReceiveBeginPlay`)
  (add `self.OnMatchStarted` (delegate `ChangeTeams`))
  (add `self.OnMatchEnded` (delegate `StopChangingTeams`))
  (add `self.OnPlayerWinsGame` (delegate `PlayerWon`))
  (add `self.OnPlayerLoggedIn` (delegate `AddPLayerConnnected`)))

(event `ChangeTeams`
  (if (`KismetArrayLibrary.Array_Contains` (`.GameRules` (break `WinConditionSettings` (`.WinConditions` (break `GameModeSettings` (`self.CurrentGameModeSettings`))))) "ChangeTeamEveryXSeconds")
    (bind _returnvalue (`KismetSystemLibrary.K2_SetTimerDelegate` (delegate `CustomEvent`) (`self.ChangeTeamsSeconds`) true))
    (set `self.ChangeTeamsTimerHandle` _returnvalue)))

(event `StopChangingTeams`
  (`KismetSystemLibrary.K2_ClearAndInvalidateTimerHandle` (`self.ChangeTeamsTimerHandle`)))

(event `AddPLayerConnnected` :!signature `self.OnPlayerLoggedIn`
  (params (PlayerController :type "PBPlayerController Object Reference"))
  (`/Engine/EditorBlueprintResources/StandardMacros.IncrementInt` (`self.ConnectedPlayers`)))

(event `PlayerWon` :!signature `self.OnPlayerWinsGame`
  (params (PlayerCharacter :type "PBCharacter Object Reference"))
  (`KismetArrayLibrary.Array_AddUnique` (`self.WinnerCharacters`) PlayerCharacter)
  (`/Engine/EditorBlueprintResources/StandardMacros.DoOnce` false
    (:`Completed`
      (add `self.OnMatchEnded` (delegate `ShowWin`)))))

(event `ShowWin`
  (bind _outactors (`GameplayStatics.GetAllActorsOfClass` "/Game/PC_Base.PC_Base_C"))
  (for _array_element _outactors
    (`/Game/PC_Base.ClientShowGameWonScreen` _array_element)))

(event `CustomEvent`
  (`self.ChangePlayersTeams`))

(fn `UserConstructionScript`)