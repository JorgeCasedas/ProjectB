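; PC_Base is a player controller Blueprint that puts match UI on screen.
; On BeginPlay it calls the parent and binds to the match-started event, with a handler that adds the in-game abilities widget to the viewport.
; Pressing G reads the new game mode and rules from GI_Base, shows them in a WBP_NewGameMode widget, and removes it after a short timer.
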(event `self.ReceiveBeginPlay`
  (`parent.ReceiveBeginPlay`)
  (add `self.OnMatchStarted` (`|CreateDelegate` :!event `MatchStartedBP`)))

(event `MatchStartedBP`
  (bind _returnvalue (`|CreateWidget` "/Game/Widgets/WBP_InGameAbilities.WBP_InGameAbilities_C"))
  (`UserWidget.AddToViewport` _returnvalue 0))

(event `Key|G`
  (params (Key :type "Key Structure"))
  (:`Pressed`
    (bind _asgi_base (cast `/Game/GI_Base` (`GameplayStatics.GetGameInstance`)))
    (bind _fgamemodesettings (`/Game/GI_Base.GetNewGameModeAndRules` _asgi_base))
    (bind _returnvalue (`|CreateWidget` "/Game/Widgets/WBP_NewGameMode.WBP_NewGameMode_C" null _fgamemodesettings))
    (`UserWidget.AddToViewport` _returnvalue 0)
    (`KismetSystemLibrary.K2_SetTimerDelegate` (delegate `RemoveWidget`) 2.0)))

(event `RemoveWidget`
  (`Widget.RemoveFromParent` (stale `Key|G` _returnvalue)))

(fn `UserConstructionScript`)